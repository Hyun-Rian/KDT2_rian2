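; BP_MyBox2 is a trigger box that starts the game's moving stairs and rects the first time its static mesh is hit.
; The hit, gated by the Onetime flag, prints "Game Start", sets the play flag on every BP_MovingstairRL, BP_MovingstairRect and BP_MoveRect, then clears the flag.
; Overlap begin and end only print debug strings; the loops toggling BP_MoveRect play on and off are left disconnected.
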(event OnComponentBeginOverlap(StaticMesh)
  (params (OverlappedComponent :type Primitive%20Component%20Object%20Reference) (OtherActor :type Actor%20Object%20Reference) (OtherComp :type Primitive%20Component%20Object%20Reference) (OtherBodyIndex :type Integer) (bFromSweep :type Boolean) (SweepResult :type Hit%20Result%20Structure%20%28by%20ref%29))
  (Development|PrintString "MoveChair"))

(event OnComponentEndOverlap(StaticMesh)
  (params (OverlappedComponent :type Primitive%20Component%20Object%20Reference) (OtherActor :type Actor%20Object%20Reference) (OtherComp :type Primitive%20Component%20Object%20Reference) (OtherBodyIndex :type Integer))
  (Development|PrintString "StopChair"))

(event OnComponentHit(StaticMesh)
  (params (HitComponent :type Primitive%20Component%20Object%20Reference) (OtherActor :type Actor%20Object%20Reference) (OtherComp :type Primitive%20Component%20Object%20Reference) (NormalImpulse :type Vector :default "0, 0, 0") (Hit :type Hit%20Result%20Structure%20%28by%20ref%29))
  (if (Variables|Default|Getonetime)
    (Development|PrintString "Game Start" true true "(R=0.000000,G=0.660000,B=1.000000,A=1.000000)" 5.0)
    (bind _outactors (Actor|GetAllActorsOfClass "/Game/Myprecontents/BluePrint/BP_MovingstairRL.BP_MovingstairRL_C"))
    (for _array_element _outactors
      (Variables|/Game/Myprecontents/BluePrint/BP_MovingstairRL.BP_MovingstairRL_C|SetIsplay _array_element true))
    (bind _outactors_2 (Actor|GetAllActorsOfClass "/Game/Myprecontents/BluePrint/BP_MovingstairRect.BP_MovingstairRect_C"))
    (for _array_element_2 _outactors_2
      (Variables|/Game/Myprecontents/BluePrint/BP_MovingstairRect.BP_MovingstairRect_C|SetIsplay _array_element_2 true))
    (bind _outactors_3 (Actor|GetAllActorsOfClass "/Game/Myprecontents/BluePrint/BP_MoveRect.BP_MoveRect_C"))
    (for _array_element_3 _outactors_3
      (Variables|/Game/Myprecontents/BluePrint/BP_MoveRect.BP_MoveRect_C|SetIsPlay _array_element_3 true))
    (Variables|Default|Setonetime false)))

(fn ConstructionScript)