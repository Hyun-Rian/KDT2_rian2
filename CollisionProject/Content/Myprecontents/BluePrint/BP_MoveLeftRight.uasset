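; BP_MoveLeftRight is an actor whose Sphere component shuttles back and forth along its relative X axis.
; While IsPlay is set, Tick moves it by Speed scaled by delta time and flips IsMoveRight at the fixed bounds of 0 and 1000.
; EventPlay and EventStop toggle IsPlay to start and pause the motion.
; An unconnected copy of the movement logic, without delta-time scaling, never runs.
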(event EventEventPlay
  (Variables|Default|SetIsPlay true))

(event EventEventStop
  (Variables|Default|SetIsPlay false))

(event EventTick
  (params (DeltaSeconds :type Float%20%28single-precision%29))
  (bind _sphere (Variables|Default|GetSphere))
  (bind _sphere_2 (Variables|Default|GetSphere))
  (if (Variables|Default|GetIsPlay)
    (if (Variables|Default|GetIsMoveRight)
      ;[1 0.9554 0.4538 1 30] x축 speed만큼 이동(오른쪽)
      (Transformation|AddRelativeLocation _sphere_2 (Math|Vector|MakeVector (* DeltaSeconds (Variables|Default|GetSpeed)) 0.0 0.0) false false)
      (if (>= (.x (Variables|/Script/Engine.SceneComponent|GetRelativeLocation _sphere_2)) 1e+03)
        (Variables|Default|SetIsMoveRight false))
      (else
        ;[0.5787 1 0.9401 1 30] x축 -speed만큼 이동(왼쪽)
        (Transformation|AddRelativeLocation _sphere (Math|Vector|MakeVector (* (* DeltaSeconds (Variables|Default|GetSpeed)) -1.0) 0.0 0.0) false false)
        (if (<= (.x (Variables|/Script/Engine.SceneComponent|GetRelativeLocation _sphere)) 0.0)
          (Variables|Default|SetIsMoveRight true))))))

(fn ConstructionScript)