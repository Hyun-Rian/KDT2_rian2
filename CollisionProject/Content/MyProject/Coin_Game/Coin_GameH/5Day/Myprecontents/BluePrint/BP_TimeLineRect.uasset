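; BP_TimeLineRect is a Timeline test Blueprint that slides a Cube along relative X, scaled by Distance, using debug keys.
; Holding P plays or reverses the Timeline, flipping IsRight on each finish to ping-pong until release stops it.
; K, L and O exercise play from start, reverse from end and SetNewTime.
; A four-direction rectangular path using MoveType and Move functions is left unconnected, as is EnableInput.
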(event EventBeginPlay)

(event Input|KeyboardEvents|P
  (params (Key :type Key%20Structure))
  (:Pressed
    (if (Variables|Default|GetIsRight) :!label _label
      (bind _새_트랙_0 (Timeline|타임라인 Play)
        (:Update
          (Transformation|SetRelativeLocation (Variables|Default|GetCube) (Math|Vector|MakeVector (* _새_트랙_0 (Variables|Default|GetDistance)) 0.0 0.0) false false))
        (:Finished
          (Variables|Default|SetIsRight (not (Variables|Default|GetIsRight)))
          (goto _label)))
      (else
        (Timeline|타임라인 Reverse))))
  (:Released
    (Timeline|타임라인 Stop)))

(event Input|KeyboardEvents|K
  (params (Key :type Key%20Structure))
  (:Pressed
    (bind _새_트랙_0 (Timeline|타임라인 PlayFromStart)
      (:Update
        (Transformation|SetRelativeLocation (Variables|Default|GetCube) (Math|Vector|MakeVector (* _새_트랙_0 (Variables|Default|GetDistance)) 0.0 0.0) false false))
      (:Finished
        (Variables|Default|SetIsRight (not (Variables|Default|GetIsRight)))
        (if (Variables|Default|GetIsRight)
          (Timeline|타임라인 Play)
          (else
            (Timeline|타임라인 Reverse)))))))

(event Input|KeyboardEvents|L
  (params (Key :type Key%20Structure))
  (:Pressed
    (bind _새_트랙_0 (Timeline|타임라인 ReverseFromEnd)
      (:Update
        (Transformation|SetRelativeLocation (Variables|Default|GetCube) (Math|Vector|MakeVector (* _새_트랙_0 (Variables|Default|GetDistance)) 0.0 0.0) false false))
      (:Finished
        (Variables|Default|SetIsRight (not (Variables|Default|GetIsRight)))
        (if (Variables|Default|GetIsRight)
          (Timeline|타임라인 Play)
          (else
            (Timeline|타임라인 Reverse)))))))

(event Input|KeyboardEvents|O
  (params (Key :type Key%20Structure))
  (:Pressed
    (bind _새_트랙_0 (Timeline|타임라인 SetNewTime)
      (:Update
        (Transformation|SetRelativeLocation (Variables|Default|GetCube) (Math|Vector|MakeVector (* _새_트랙_0 (Variables|Default|GetDistance)) 0.0 0.0) false false))
      (:Finished
        (Variables|Default|SetIsRight (not (Variables|Default|GetIsRight)))
        (if (Variables|Default|GetIsRight)
          (Timeline|타임라인 Play)
          (else
            (Timeline|타임라인 Reverse)))))))

(fn ConstructionScript)

(fn MoveRight
  (params (DeltaLocation_X :type Float%20%28double-precision%29))
  (bind _cube (Variables|Default|GetCube))
  (Transformation|SetRelativeLocation _cube (Math|Vector|MakeVector DeltaLocation_X 0.0 0.0) false false)
  (if (>= (.x (Variables|/Script/Engine.SceneComponent|GetRelativeLocation _cube)) 5e+02)
    (Variables|Default|SetMoveType "NewEnumerator1")))

(fn MoveUp
  (params (DeltaLocation_Z :type Float%20%28double-precision%29))
  (Transformation|SetRelativeLocation (Variables|Default|GetCube) (Math|Vector|MakeVector 0.0 0.0 DeltaLocation_Z) false false))

(fn MoveLeft
  (params (A :type Float%20%28double-precision%29))
  (bind _cube (Variables|Default|GetCube))
  (Transformation|SetRelativeLocation _cube (Math|Vector|MakeVector (* A -1.0) 0.0 0.0) false false)
  (if (<= (.x (Variables|/Script/Engine.SceneComponent|GetRelativeLocation _cube)) 0.0)
    (Variables|Default|SetMoveType "NewEnumerator3")))

(fn MoveDown
  (params (A :type Float%20%28double-precision%29))
  (bind _cube (Variables|Default|GetCube))
  (Transformation|SetRelativeLocation _cube (Math|Vector|MakeVector 0.0 0.0 (* A -1.0)) false false)
  (if (<= (.z (Variables|/Script/Engine.SceneComponent|GetRelativeLocation _cube)) 0.0)
    (Variables|Default|SetMoveType "NewEnumerator0")))