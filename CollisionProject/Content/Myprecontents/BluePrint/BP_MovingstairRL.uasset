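; Moving stair Blueprint that slides its Cube component back and forth along relative X while Isplay is true.
; Tick scales Speed by delta time and calls MoveRight or MoveLeft based on MoveRL, which each function flips at its hard-coded travel limit.
; MoveUp and MoveDown provide matching Z movement, but Tick never calls them and their limit checks do nothing.
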(event EventTick
  (params (DeltaSeconds :type Float%20%28single-precision%29))
  (bind _speed (Variables|Default|GetSpeed))
  (bind _returnvalue (* DeltaSeconds _speed))
  (if (Variables|Default|GetIsplay)
    (if (Variables|Default|GetMoveR-L)
      (CallFunction|MoveRight _returnvalue)
      (else
        (CallFunction|MoveLeft _returnvalue)))))

(fn ConstructionScript)

(fn MoveRight
  (params (DeltaLocation_X :type Float%20%28double-precision%29))
  (bind _cube (Variables|Default|GetCube))
  (Transformation|AddRelativeLocation _cube (Math|Vector|MakeVector DeltaLocation_X 0.0 0.0) false false)
  (if (>= (.x (Variables|/Script/Engine.SceneComponent|GetRelativeLocation _cube)) 5e+02)
    (Variables|Default|SetMoveR-L false)))

(fn MoveUp
  (params (DeltaLocation_Z :type Float%20%28double-precision%29))
  (bind _cube (Variables|Default|GetCube))
  (Transformation|AddRelativeLocation _cube (Math|Vector|MakeVector 0.0 0.0 DeltaLocation_Z) false false)
  (if (>= (.z (Variables|/Script/Engine.SceneComponent|GetRelativeLocation _cube)) 5e+02)
    _))

(fn MoveLeft
  (params (A :type Float%20%28double-precision%29))
  (bind _cube (Variables|Default|GetCube))
  (Transformation|AddRelativeLocation _cube (Math|Vector|MakeVector (* A -1.0) 0.0 0.0) false false)
  (if (<= (.x (Variables|/Script/Engine.SceneComponent|GetRelativeLocation _cube)) 0.0)
    (Variables|Default|SetMoveR-L true)))

(fn MoveDown
  (params (a :type Float%20%28double-precision%29))
  (bind _cube (Variables|Default|GetCube))
  (Transformation|AddRelativeLocation _cube (Math|Vector|MakeVector 0.0 0.0 (* a -1.0)) false false)
  (if (<= (.z (Variables|/Script/Engine.SceneComponent|GetRelativeLocation _cube)) 0.0)
    _))