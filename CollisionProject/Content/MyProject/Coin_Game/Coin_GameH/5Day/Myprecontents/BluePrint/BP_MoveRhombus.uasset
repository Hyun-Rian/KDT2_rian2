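; Moving actor Blueprint whose static mesh travels along diagonal legs in the relative X-Z plane, shaped as a rhombus.
; While IsPlay is set, Tick switches on the MoveVector enum and calls one of four move functions with a step scaled by Speed and delta time.
; Each function offsets the mesh and sets MoveVector upon reaching its X or Z limit.
; EventPlay and EventStop toggle the movement.
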(event EventEventStop
  (Variables|Default|SetIsPlay false))

(event EventEventPlay
  (Variables|Default|SetIsPlay true))

(event EventTick
  (params (DeltaSeconds :type Float%20%28single-precision%29))
  (bind _speed (Variables|Default|Getspeed))
  (bind _returnvalue (* DeltaSeconds _speed))
  (if (Variables|Default|GetIsPlay)
    (switch Utilities|FlowControl|Switch|SwitchonEN_MoveXY_Type (Variables|Default|GetMoveVector)
      (:NewEnumerator0
        (CallFunction|MoveXY _returnvalue _returnvalue))
      (:NewEnumerator1
        (CallFunction|Move-XY _returnvalue _returnvalue))
      (:NewEnumerator2
        (CallFunction|Move-X-Y _returnvalue))
      (:NewEnumerator3
        (CallFunction|MoveX-Y _returnvalue _returnvalue)))))

(fn ConstructionScript)

(fn MoveXY
  (params (DeltaLocation_X :type Float%20%28double-precision%29) (DeltaLocation_Z :type Float%20%28double-precision%29))
  (bind _staticmesh (Variables|Default|GetStaticMesh))
  (Transformation|AddRelativeLocation _staticmesh (Math|Vector|MakeVector DeltaLocation_X 0.0 DeltaLocation_Z) false false)
  (if (>= (.x (Variables|/Script/Engine.SceneComponent|GetRelativeLocation _staticmesh)) 5e+02)
    (Variables|Default|SetMoveVector "NewEnumerator1")))

(fn Move-XY
  (params (DeltaLocation_Z :type Float%20%28double-precision%29) (A :type Float%20%28double-precision%29))
  (bind _staticmesh (Variables|Default|GetStaticMesh))
  (Transformation|AddRelativeLocation _staticmesh (Math|Vector|MakeVector (* A -1.0) 0.0 DeltaLocation_Z) false false)
  (if (<= (.x (Variables|/Script/Engine.SceneComponent|GetRelativeLocation _staticmesh)) 0.0)
    (Variables|Default|SetMoveVector "NewEnumerator2")))

(fn Move-X-Y
  (params (A :type Float%20%28double-precision%29))
  (bind _returnvalue (* A -1.0))
  (bind _staticmesh (Variables|Default|GetStaticMesh))
  (Transformation|AddRelativeLocation _staticmesh (Math|Vector|MakeVector _returnvalue 0.0 _returnvalue) false false)
  (if (<= (.x (Variables|/Script/Engine.SceneComponent|GetRelativeLocation _staticmesh)) -5e+02)
    (Variables|Default|SetMoveVector "NewEnumerator3")))

(fn MoveX-Y
  (params (DeltaLocation_X :type Float%20%28double-precision%29) (A :type Float%20%28double-precision%29))
  (bind _staticmesh (Variables|Default|GetStaticMesh))
  (Transformation|AddRelativeLocation _staticmesh (Math|Vector|MakeVector DeltaLocation_X 0.0 (* A -1.0)) false false)
  (if (<= (.z (Variables|/Script/Engine.SceneComponent|GetRelativeLocation _staticmesh)) 0.0)
    (Variables|Default|SetMoveVector "NewEnumerator0")))